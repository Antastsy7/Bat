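; Sphere actor with a point light that brightens when shot and gradually fades.
; Hits from Bullet actors add a fixed step to the light intensity while it is below a maximum.
; Tick subtracts Persecond every frame while intensity exceeds that amount, without delta-time scaling, so the fade is frame-rate dependent.
; A GetClosest helper finds the component nearest a location but is not called in these graphs.
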(event EventBeginPlay)

(event Collision|EventActorBeginOverlap
  (params (OtherActor :type Actor%20Object%20Reference)))

(event EventTick
  (params (DeltaSeconds :type Float%20%28single-precision%29))
  (if (> (Variables|/Script/Engine.LightComponentBase|GetIntensity (Variables|Default|GetPointLight)) (Variables|Default|Getpersecond))
    (bind _output_get (Variables|Default|SetPointLight (Variables|Default|GetPointLight)))
    (Rendering|Components|Light|SetIntensity _output_get (- (Variables|/Script/Engine.LightComponentBase|GetIntensity _output_get) (Variables|Default|Getpersecond)))))

(event Collision|EventHit
  (params (MyComp :type Primitive%20Component%20Object%20Reference) (Other :type Actor%20Object%20Reference) (OtherComp :type Primitive%20Component%20Object%20Reference) (bSelfMoved :type Boolean) (HitLocation :type Vector :default "0, 0, 0") (HitNormal :type Vector :default "0, 0, 0") (NormalImpulse :type Vector :default "0, 0, 0") (Hit :type Hit%20Result%20Structure%20%28by%20ref%29))
  (if (== (Utilities|GetClass Other) "/Game/BP/Blueprints/Bullet.Bullet_C")
    (if (< (Variables|/Script/Engine.LightComponentBase|GetIntensity (Variables|Default|GetPointLight)) (Variables|Default|GetMaxvalue))
      (bind _output_get (Variables|Default|SetPointLight (Variables|Default|GetPointLight)))
      (Rendering|Components|Light|SetIntensity _output_get (+ (Variables|/Script/Engine.LightComponentBase|GetIntensity _output_get) (Variables|Default|GetAddon))))))

(fn ConstructionScript)

(fn GetClosest
  (params (location :type Vector))
  (bind _output_get (LocalVariables|SetMin 1e+07))
  (for _array_element 0
    (if (< (Math|Vector|Distance(Vector) location (Transformation|GetWorldLocation _array_element)) _output_get)
      (LocalVariables|SetMin (Math|Vector|Distance(Vector) location (Transformation|GetWorldLocation _array_element)))
      (LocalVariables|Settarget _array_element)))
  (return (LocalVariables|Gettarget)))