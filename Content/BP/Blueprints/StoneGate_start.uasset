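; StoneGate_start is a stone gate that, once Activate is called, sinks at a steady rate while playing audio.
; Tick moves the static mesh downward while active, and a looping timer repeatedly spawns expanding SoundWave actors at the gate's location.
; After a few seconds Complete stops the movement, fades out the audio and clears the Sound timer, though its own looping timer is never cleared.
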(event Custom|Activate
  (Variables|Default|SetActive true)
  (bind _returnvalue (AddComponent|AddAudioComponent false))
  (Audio|Components|Audio|Play _returnvalue 0.0)
  (Variables|Default|SetAudio _returnvalue)
  (bind _returnvalue_2 (Utilities|Time|SetTimerbyFunctionName 0 "Sound" 0.5 true))
  (Variables|Default|SetTimer _returnvalue_2)
  (Utilities|Time|SetTimerbyFunctionName 0 "Complete" 5.0 true))

(event EventBeginPlay)

(event Collision|EventActorBeginOverlap
  (params (OtherActor :type Actor%20Object%20Reference)))

(event EventTick
  (params (DeltaSeconds :type Float%20%28single-precision%29))
  (if (Variables|Default|GetActive)
    (Transformation|AddWorldOffset (Variables|Debug|GetStaticMeshComponent) (* "0.000000,0.000000,-90.000000" DeltaSeconds) false false)))

(fn ConstructionScript)

(fn Sound
  (bind _returnvalue (Game|SpawnActorfromClass "/Game/BP/SoundWaves/SoundWave.SoundWave_C" (Math|Conversions|ToTransform(Vector) (Transformation|GetActorLocation)) "Undefined" 0 0))
  (Default|SetVariables _returnvalue 2.0 1e+02 "0, 0, 0" true 1.5))

(fn Complete
  (Variables|Default|SetActive false)
  (Audio|Components|Audio|FadeOut (Variables|Default|GetAudio) 2.0 0.0 "Linear" :!class /Script/Engine.AudioComponent)
  (Utilities|Time|ClearandInvalidateTimerbyHandle (Variables|Default|GetTimer)))