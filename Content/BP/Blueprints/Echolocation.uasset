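; Echolocation is a game-flow Blueprint that handles a fire-ending story event, headset detection and quitting on Escape.
; FireEnds sets the passed Dragon fading, removes the Block actor, and switches the Dog's WildDog_AI controller to pet behavior.
; BeginPlay clears the Text flag when no HMD is enabled, but the logic revealing Instruction-tagged actors from that flag is unconnected.
; DeerEscaped and the construction script are empty.
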(event EventBeginPlay
  (if (not (Class|HeadMountedDisplayFunctionLibrary|IsHeadMountedDisplayEnabled))
    (Variables|Default|SetText false)))

(event Input|KeyboardEvents|Escape
  (params (Key :type Key%20Structure :default "None"))
  (:Pressed
    (Game|QuitGame 0 "Quit" false)))

(fn ConstructionScript)

(fn FireEnds
  (params (Dragon :type Pawn%20Object%20Reference))
  (bind _asdragon (Utilities|Casting|CastToDragon Dragon))
  (Variables|/Game/BP/Dragon/Dragon.Dragon_C|SetFading _asdragon true)
  (bind _returnvalue (Actor|GetActorOfClass "/Game/BP/Dragon/Block.Block_C"))
  (Default|BlockRemove _returnvalue)
  (bind _returnvalue_2 (Actor|GetActorOfClass "/Game/BP/Pets/Dog.Dog_C"))
  (bind _aswild_dog_ai (Utilities|Casting|CastToWildDog_AI (AI|GetAIController _returnvalue_2)))
  (Default|ChangetoPet _aswild_dog_ai))

(fn DeerEscaped)