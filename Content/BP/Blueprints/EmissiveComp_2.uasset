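; Actor component that makes the owner's skeletal mesh react to overlaps with actors tagged SoundWave through a material effect, likely an emissive glow.
; On BeginPlay it finds the mesh and binds its begin-overlap event, where a tagged hit boosts Strength toward a cap via ChangeVal.
; Tick uses the same helper to ease Strength toward zero and writes it to the mesh's "Strength" material parameter.
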(event Custom|Overlap
  (params (OverlappedComponent :type Primitive%20Component%20Object%20Reference) (OtherActor :type Actor%20Object%20Reference) (OtherComp :type Primitive%20Component%20Object%20Reference) (OtherBodyIndex :type Integer) (bFromSweep :type Boolean) (SweepResult :type Hit%20Result%20Structure%20%28by%20ref%29))
  (if (Actor|ActorHasTag OtherActor "SoundWave")
    (bind _returnvalue (Class|Savetxt|ChangeVal (Variables|Default|GetStrength) 1.5 2.0 true))
    (Variables|Default|SetStrength _returnvalue)))

(event EventBeginPlay
  (bind _returnvalue (Components|GetOwner))
  (bind _returnvalue_2 (Actor|GetComponentbyClass _returnvalue "/Script/Engine.SkeletalMeshComponent"))
  (Variables|Default|SetSKMesh _returnvalue_2)
  (Components|Tick|SetComponentTickEnabled true)
  (Collision|AssignOnComponentBeginOverlap _returnvalue_2 (delegate Custom|Overlap)))

(event EventTick
  (params (DeltaSeconds :type Float%20%28single-precision%29))
  (bind _returnvalue (Class|Savetxt|ChangeVal (Variables|Default|GetStrength) 0.02 0.0 false))
  (bind _output_get (Variables|Default|SetStrength _returnvalue))
  (Rendering|Material|SetScalarParameterValueonMaterials (Variables|Default|GetSKMesh) "Strength" _output_get))