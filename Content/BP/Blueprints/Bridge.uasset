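; Bridge actor that, once activated, raises a row of cube segments one at a time to form a bridge.
; The construction script builds Length-driven, evenly spaced flattened static mesh components along X and stores them in Cubes.
; BridgeActivated starts a looping timer that selects the next cube and plays a floating sound, while Tick lifts it at Height/Frequency speed.
; After the last segment, movement stops and Complete is called once.
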(event Custom|BridgeActivated
  (Variables|Default|SetActivate true)
  (bind _returnvalue (Utilities|Time|SetTimerbyEvent (delegate Custom|FloatUp) (Variables|Default|GetFrequency) true))
  (Variables|Default|SetTimer _returnvalue))

(event Custom|FloatUp
  (bind _result (Math|Integer|IncrementInt (Variables|Default|GetIndex))
    (:%20%20
      (if (<= _result (Variables|Default|GetLength))
        (Variables|Default|SetCurrentCube (Utilities|Array|Get(acopy) (Variables|Default|GetCubes) (Variables|Default|GetIndex)))
        (Audio|PlaySoundatLocation "/Game/Audio/BridgeFloating.BridgeFloating" (Transformation|GetActorLocation) "0, 0, 0" 1.0 1.0 0.0 0 0 0)
        (else
          (Variables|Default|SetActivate false)
          (Utilities|FlowControl|DoOnce false
            (:Completed
              (Default|CallComplete))))))))

(event EventBeginPlay)

(event Collision|EventActorBeginOverlap
  (params (OtherActor :type Actor%20Object%20Reference)))

(event EventTick
  (params (DeltaSeconds :type Float%20%28single-precision%29))
  (if (Variables|Default|GetActivate)
    (Utilities|IsValid (Variables|Default|GetCurrentCube)
      (:Is%20Valid
        (Transformation|AddWorldOffset (Variables|Default|GetCurrentCube) (Math|Vector|MakeVector 0.0 0.0 (* DeltaSeconds (/ (Variables|Default|GetHeight) (Variables|Default|GetFrequency)))) false false)))))

(fn ConstructionScript
  (for _index (range 0 (Variables|Default|GetLength))
    (bind _returnvalue (AddComponent|AddStaticMeshComponent false (Math|Transform|MakeTransform (Math|Vector|MakeVector (* _index 1.1e+02) 0.0 0.0) "0, 0, 0" "1.000000,1.700000,0.200000")))
    (Utilities|Array|SetArrayElem (Variables|Default|GetCubes) _index _returnvalue true)))