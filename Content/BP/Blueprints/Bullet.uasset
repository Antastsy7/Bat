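; Bullet actor that destroys itself three seconds after spawning or upon its second hit, whichever comes first.
; BeginPlay resets a hit counter and starts the timeout, while each Hit increments the counter through a branch with empty paths.
; Disconnected, never-run logic would brighten the closest light on a hit Structure or add a point light to the hit actor.
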(event EventBeginPlay
  (Variables|Default|SetCount 0)
  (Utilities|FlowControl|Delay 3.0)
  (Actor|DestroyActor))

(event EventTick
  (params (DeltaSeconds :type Float%20%28single-precision%29)))

(event Collision|EventHit
  (params (MyComp :type Primitive%20Component%20Object%20Reference) (Other :type Actor%20Object%20Reference) (OtherComp :type Primitive%20Component%20Object%20Reference) (bSelfMoved :type Boolean) (HitLocation :type Vector :default "0, 0, 0") (HitNormal :type Vector :default "0, 0, 0") (NormalImpulse :type Vector :default "0, 0, 0") (Hit :type Hit%20Result%20Structure%20%28by%20ref%29))
  (if (== (Variables|Default|GetCount) 0)
    _
    (else
      _))
  (bind _result (Math|Integer|IncrementInt (Variables|Default|GetCount))
    (:%20%20
      (if (>= _result 2)
        (Actor|DestroyActor)))))

(fn ConstructionScript)