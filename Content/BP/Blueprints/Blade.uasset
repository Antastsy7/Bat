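; Blade is a grabbable weapon that stabs deer.
; It sets a fixed grip on its static mesh at BeginPlay; releasing it hides and disarms it and teleports it to the world origin.
; While active, overlapping a Deer2 calls GetHit on its Deer_AI2 controller, plays a stab sound and clears Active without hiding the mesh, allowing one hit per activation.
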(event OnComponentBeginOverlap(StaticMesh)
  (params (OverlappedComponent :type Primitive%20Component%20Object%20Reference) (OtherActor :type Actor%20Object%20Reference) (OtherComp :type Primitive%20Component%20Object%20Reference) (OtherBodyIndex :type Integer) (bFromSweep :type Boolean) (SweepResult :type Hit%20Result%20Structure%20%28by%20ref%29))
  (if (Variables|Default|GetActive)
    (bind _asdeer_2 (Utilities|Casting|CastToDeer2 OtherActor))
    (bind _asdeer_ai2 (Utilities|Casting|CastToDeer_AI2 (Pawn|GetController _asdeer_2)))
    (Default|GetHit _asdeer_ai2)
    (Variables|Default|SetActive false)
    (Audio|PlaySoundatLocation "/Game/Audio/Stab.Stab" (Transformation|GetActorLocation) "0, 0, 0" 1.0 1.0 0.0 0 0 0)))

(event Custom|Released
  (CallFunction|SetActive false)
  (Transformation|SetActorTransform (Math|Transform|MakeTransform "0, 0, 0") false true))

(event EventBeginPlay
  (Default|SetFixedGrab :self (Variables|Default|GetGrabable) :Volume (Variables|Default|GetStaticMesh) :Animation "/Game/Model/Animations/Grabs/grab_round_medium.grab_round_medium")
  (EventDispatchers|BindEventtoReleaseNotify (Variables|Default|GetGrabable) (delegate Custom|Released)))

(event Collision|EventActorBeginOverlap
  (params (OtherActor :type Actor%20Object%20Reference)))

(event EventTick
  (params (DeltaSeconds :type Float%20%28single-precision%29)))

(fn ConstructionScript)

(fn SetActive
  (params (Active :type Boolean))
  (Variables|Default|SetActive Active)
  (Rendering|SetVisibility (Variables|Default|GetStaticMesh) Active false))