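; Altar table Blueprint that accepts an animal offering matching its Type (Rabbit, Deer or Bear) and signals that the altar is activated.
; On mesh overlap, a dead rabbit snaps to the plate, while a released deer or bear heart of matching type snaps to the scene component.
; Each path stops physics and fires once.
; Unconnected leftover logic sketches a blood decal and growing spline-mesh effect.
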(event OnComponentBeginOverlap(StaticMeshComponent)
  (params (OverlappedComponent :type Primitive%20Component%20Object%20Reference) (OtherActor :type Actor%20Object%20Reference) (OtherComp :type Primitive%20Component%20Object%20Reference) (OtherBodyIndex :type Integer) (bFromSweep :type Boolean) (SweepResult :type Hit%20Result%20Structure%20%28by%20ref%29))
  (switch Utilities|FlowControl|Switch|SwitchonAnimalType (Variables|Default|GetType)
    (:NewEnumerator0
      (bind _asdead_rabbit (Utilities|Casting|CastToDeadRabbit OtherActor))
      (Utilities|FlowControl|DoOnce false
        (:Completed
          (Physics|SetSimulatePhysics (Variables|/Game/BP/Rabbit/DeadRabbit.DeadRabbit_C|GetSkeletalMesh _asdead_rabbit) false)
          (Transformation|AttachComponentToComponent _asdead_rabbit (Variables|Default|GetPlate) "None" "SnapToTarget" "KeepRelative" "KeepWorld" true)
          (Default|CallAlterActivated))))
    (:NewEnumerator1
      (bind _asheart (Utilities|Casting|CastToHeart OtherActor :!label _label))
      (if (and (not (Variables|/Game/BP/Heart/Heart.Heart_C|GetGrab _asheart)) (Utilities|Enum|Equal(Enum) (Variables|/Game/BP/Heart/Heart.Heart_C|GetType _asheart) (Variables|Default|GetType)))
        (Utilities|FlowControl|DoOnce false
          (:Completed
            (Physics|SetSimulatePhysics (Variables|/Game/BP/Heart/Heart.Heart_C|GetSphere _asheart) false)
            (Actor|Tick|SetActorTickEnabled _asheart)
            (Transformation|AttachComponentToComponent _asheart (Variables|Default|GetScene) "None" "SnapToTarget" "KeepRelative" "KeepWorld" true)
            (Default|CallAlterActivated)))
        (else
          (Development|PrintString "????"))))
    (:NewEnumerator2
      (goto _label))))

(event EventBeginPlay)

(event EventTick
  (params (DeltaSeconds :type Float%20%28single-precision%29)))

(fn ConstructionScript)