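; Belltower actor that emits expanding sound waves while a DeadRabbit rests in its Box trigger.
; The rabbit's overlap starts a looping timer that spawns a configured SoundWave actor and plays a sound, and its exit clears the timer.
; Each pulse resets a Strength value, overlapping SoundWave-tagged actors raise it, and Tick applies Decay and feeds it to tower and altar materials.
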(event OnComponentBeginOverlap(Box)
  (params (OverlappedComponent :type Primitive%20Component%20Object%20Reference) (OtherActor :type Actor%20Object%20Reference) (OtherComp :type Primitive%20Component%20Object%20Reference) (OtherBodyIndex :type Integer) (bFromSweep :type Boolean) (SweepResult :type Hit%20Result%20Structure%20%28by%20ref%29))
  (Utilities|FlowControl|Sequence
    (:then_0
      (if (not (Variables|Default|GetIsActive))
        (bind _asdead_rabbit (Utilities|Casting|CastToDeadRabbit OtherActor))
        (Variables|Default|SetDead _asdead_rabbit)
        (CallFunction|Activate)))
    (:then_1
      (if (Actor|ActorHasTag OtherActor "SoundWave")
        (bind _returnvalue (Class|Savetxt|ChangeVal (Variables|Default|GetStrength) 1.0 2.0 true))
        (Variables|Default|SetStrength _returnvalue)))))

(event OnComponentEndOverlap(Box)
  (params (OverlappedComponent :type Primitive%20Component%20Object%20Reference) (OtherActor :type Actor%20Object%20Reference) (OtherComp :type Primitive%20Component%20Object%20Reference) (OtherBodyIndex :type Integer))
  (if (and (== OtherActor (Variables|Default|GetDead)) (Variables|Default|GetIsActive))
    (Variables|Default|SetDead 0)
    (CallFunction|Deactivate)))

(event Custom|SendSoundWave
  (bind _returnvalue (Game|SpawnActorfromClass "/Game/BP/SoundWaves/SoundWave.SoundWave_C" (Math|Conversions|ToTransform(Vector) (Transformation|GetActorLocation)) "Undefined" 0 0))
  (Default|SetVariables _returnvalue (Variables|Default|GetExpRate) (Variables|Default|GetMaxScale) (Variables|Default|GetDirection) true (Variables|Default|GetAddon))
  (Variables|Default|SetStrength 1.0)
  (Audio|PlaySoundatLocation (Variables|Default|GetSoundWAve) (Transformation|GetActorLocation) "0, 0, 0" 1.0 1.0 0.0 0 0 0))

(event Custom|Activate
  (bind _returnvalue (Utilities|Time|SetTimerbyEvent (delegate Custom|SendSoundWave) (Variables|Default|GetInterval) true))
  (Variables|Default|SetTimer _returnvalue)
  (Variables|Default|SetIsActive true))

(event Custom|Deactivate
  (Utilities|Time|ClearandInvalidateTimerbyHandle (Variables|Default|GetTimer))
  (Variables|Default|SetIsActive false))

(event EventBeginPlay)

(event Collision|EventActorBeginOverlap
  (params (OtherActor :type Actor%20Object%20Reference)))

(event EventTick
  (params (DeltaSeconds :type Float%20%28single-precision%29))
  (bind _returnvalue (Class|Savetxt|ChangeVal (Variables|Default|GetStrength) (* DeltaSeconds (Variables|Default|Getdecay)) 0.0 false))
  (bind _output_get (Variables|Default|SetStrength _returnvalue))
  (Rendering|Material|SetScalarParameterValueonMaterials (Variables|Debug|GetStaticMeshComponent) "Strength" _output_get)
  (Rendering|Material|SetScalarParameterValueonMaterials (Variables|Default|GetAltar) "Strength" _output_get))

(fn ConstructionScript)