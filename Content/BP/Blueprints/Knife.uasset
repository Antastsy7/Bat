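; Knife actor that the player can grab, with a fixed medium round grip on its static mesh.
; On release it deactivates, hiding the mesh and teleporting to the world origin, then calls GetKnives on the player's Hunter pawn.
; SetActive stores the state and moves the knife to origin whether activating or deactivating.
; Without a headset enabled, a Hunter overlapping it gets its UI shown, plus a debug print.
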(event Custom|Released
  (CallFunction|SetActive false)
  (bind _ashunter (Utilities|Casting|CastToHunter (Game|Player|GetPlayerPawn 0)))
  (Default|GetKnives _ashunter))

(event EventBeginPlay
  (Default|SetFixedGrab :self (Variables|Default|GetGrabable) :Volume (Variables|Default|GetStaticMesh) :Animation "/Game/Model/Animations/Grabs/grab_round_medium.grab_round_medium")
  (EventDispatchers|BindEventtoReleaseNotify (Variables|Default|GetGrabable) (delegate Custom|Released)))

(event Collision|EventActorBeginOverlap
  (params (OtherActor :type Actor%20Object%20Reference))
  (if (not (Class|HeadMountedDisplayFunctionLibrary|IsHeadMountedDisplayEnabled))
    (bind _ashunter (Utilities|Casting|CastToHunter OtherActor))
    (Widget|SetVisibility (Variables|/Game/BP/Character/Hunter.Hunter_C|GetUI _ashunter) "Visible")
    (Development|PrintString "Hello")))

(event EventTick
  (params (DeltaSeconds :type Float%20%28single-precision%29)))

(fn ConstructionScript)

(fn SetActive
  (params (Active :type Boolean))
  (Variables|Default|SetActive Active)
  (Rendering|SetVisibility (Variables|Default|GetStaticMesh) Active false)
  (Transformation|SetActorLocation "0, 0, 0" false true))